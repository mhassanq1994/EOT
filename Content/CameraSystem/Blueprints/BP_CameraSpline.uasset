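; Spline-rail camera actor that follows an activated player pawn along a camera spline paired with a player spline.
; Each tick, a recursive bisection search finds the player spline time nearest the pawn.
; The current time eases toward it, snapping on large gaps, then samples the camera spline for an interpolated position that looks at the pawn.
; Construction previews the camera at a scrub time and optionally numbers spline points, with runtime debug spheres.
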(event EventTick
  (params (DeltaSeconds :type Float%20%28single-precision%29))
  (|UpdateGroup DeltaSeconds))

(fn ConstructionScript
  (CallFunction|SetScrubCameraTime)
  (CallFunction|SetupDebugNumbers))

(fn ActivateCamera
  (params (Player :type Pawn%20Object%20Reference))
  (Utilities|IsValid Player
    (:Is%20Valid
      (bind _output_get (Variables|Default|SetPlayer%20Pawn Player))
      (Development|PrintText "PLAYER PAWN HAS BEEN SET" true true "(R=1.000000,G=0.000000,B=0.127017,A=1.000000)")
      (Development|PrintText (Utilities|Text|ToText(String) (Utilities|GetDisplayName _output_get)) true true "(R=1.000000,G=0.000000,B=0.127438,A=1.000000)"))
    (:Is%20Not%20Valid
      (Development|PrintText "PLAYER PAWN IS NOT VALID IN ACTIVATE CAMERA" true true "(R=1.000000,G=0.000000,B=0.133155,A=1.000000)"))))

(fn DeactivateCamera
  (Variables|Default|SetPlayer%20Pawn 0))

(fn SetScrubCameraTime
  (bind _splinecamera (Variables|Default|GetSplineCamera))
  (bind _constant_velocity (Variables|Spline|GetConstant%20Velocity))
  (bind _cameradebugtime (Variables|DebugTools|GetCameraDebugTime))
  (bind _splineplayer (Variables|Default|GetSplinePlayer))
  (bind _returnvalue (Spline|GetLocationatTime _splinecamera _cameradebugtime "World" _constant_velocity))
  (bind _returnvalue_2 (Spline|GetLocationatTime _splineplayer _cameradebugtime "World" _constant_velocity))
  (bind _returnvalue_3 (Math|Rotator|FindLookatRotation _returnvalue _returnvalue_2))
  (bind (_roll _pitch) (Math|Rotator|BreakRotator _returnvalue_3))
  (Transformation|SetWorldLocationAndRotation (Variables|Default|GetCamera) _returnvalue (Math|Rotator|MakeRotator _roll _pitch 0.0) false false))

(fn SetupDebugNumbers
  (if (Variables|DebugTools|GetShow%20Debug)
    (Utilities|FlowControl|Sequence
      (:then_0
        (CallFunction|AddSplineNumbers (Variables|Default|GetSplineCamera)))
      (:then_1
        (CallFunction|AddSplineNumbers (Variables|Default|GetSplinePlayer))))))

(fn AddSplineNumbers
  (params (Spline :type Spline%20Component%20Object%20Reference))
  (for _index (range (- (Spline|GetNumberOfSplinePoints Spline) 1) 0)
    (LocalVariables|Setindex _index)
    (bind _returnvalue (AddComponent|AddTextRenderComponent false (Math|Transform|MakeTransform (+ (.Location (Spline|GetLocationandTangentatSplinePoint Spline _index "Local")) "0, 0, 0") (Math|Rotator|CombineRotators (Math|Vector|RotatorfromAxisandAngle (.Tangent (Spline|GetLocationandTangentatSplinePoint Spline _index "Local")) 0.0) "0, 0, 0"))))
    (Rendering|Components|TextRender|SetText _returnvalue (Utilities|Text|ToText(Integer) (LocalVariables|Getindex)))))

(fn RecursiveDistanceCheck
  (params (Iteration :type Integer) (StartTime :type Float%20%28single-precision%29) (EndTime :type Float%20%28single-precision%29))
  (bind _constant_velocity (Variables|Spline|GetConstant%20Velocity))
  (bind _splineplayer (Variables|Default|GetSplinePlayer))
  (bind _player_pawn (Variables|Default|GetPlayer%20Pawn))
  (bind _returnvalue (Transformation|GetActorLocation _player_pawn))
  (LocalVariables|SetNum Iteration)
  (LocalVariables|SetStart StartTime)
  (LocalVariables|SetEnd EndTime)
  (LocalVariables|SetStartDistance (Math|Vector|VectorLength (- (Spline|GetLocationatTime _splineplayer (LocalVariables|GetStart) "World" _constant_velocity) _returnvalue)))
  (LocalVariables|SetEndDistance (Math|Vector|VectorLength (- (Spline|GetLocationatTime _splineplayer (LocalVariables|GetEnd) "World" _constant_velocity) _returnvalue)))
  (if (< (LocalVariables|GetStartDistance) (LocalVariables|GetEndDistance))
    (if (<= (LocalVariables|GetNum) 0)
      (LocalVariables|SetBest (LocalVariables|GetStart) :!label _label)
      (else
        (LocalVariables|SetNum (- (LocalVariables|GetNum) 1))
        (if (<= (LocalVariables|GetEndDistance) (Variables|Spline|GetDistanceThreshold))
          (goto _label)
          (else
            (bind _best_time (CallFunction|RecursiveDistanceCheck (LocalVariables|GetNum) (LocalVariables|GetStart) (Math|Float|Lerp (LocalVariables|GetStart) (LocalVariables|GetEnd) 0.5)))
            (LocalVariables|SetBest _best_time)))))
    (elif (<= (LocalVariables|GetNum) 0)
      (LocalVariables|SetBest (LocalVariables|GetEnd) :!label _label_2)
      (else
        (LocalVariables|SetNum (- (LocalVariables|GetNum) 1))
        (if (<= (LocalVariables|GetEndDistance) (Variables|Spline|GetDistanceThreshold))
          (goto _label_2)
          (else
            (bind _best_time_2 (CallFunction|RecursiveDistanceCheck (LocalVariables|GetNum) (Math|Float|Lerp (LocalVariables|GetStart) (LocalVariables|GetEnd) 0.5) (LocalVariables|GetEnd)))
            (LocalVariables|SetBest _best_time_2))))))
  (return (LocalVariables|GetBest)))

(fn UpdateDesiredTime
  (if (>= (Math|Float|Absolute(Float) (- (Variables|Spline|GetSplineDesiredTime) (Variables|Spline|GetSplineCurrentTime))) (Variables|Spline|GetTimeDifferenceThreshold))
    (Variables|Spline|SetSplineCurrentTime (Variables|Spline|GetSplineDesiredTime))
    (else
      (Variables|Spline|SetSplineCurrentTime (+ (* (- (Variables|Spline|GetSplineDesiredTime) (Variables|Spline|GetSplineCurrentTime)) (Variables|Spline|GetDeltaTime)) (Variables|Spline|GetSplineCurrentTime)))))
  (Variables|Spline|SetCameraDesiredLocation (Spline|GetLocationatTime (Variables|Default|GetSplineCamera) (Variables|Spline|GetSplineCurrentTime) "World" (Variables|Spline|GetConstant%20Velocity))))

(fn UpdateCameraPosition
  (Transformation|SetWorldLocationAndRotation (Variables|Default|GetCamera) (Math|Interpolation|VInterpTo (Transformation|GetWorldLocation (Variables|Default|GetCamera)) (Variables|Spline|GetCameraDesiredLocation) (Variables|Spline|GetDeltaTime) (Variables|Spline|GetCameraInterpSpeed)) (Math|Rotator|FindLookatRotation (Transformation|GetWorldLocation (Variables|Default|GetCamera)) (Transformation|GetActorLocation (Variables|Default|GetPlayer%20Pawn))) false false))

(fn DebugSplineMovement
  (if (Variables|DebugTools|GetShow%20Debug)
    (Rendering|Debug|DrawDebugSphere (Spline|GetLocationatTime (Variables|Default|GetSplinePlayer) (Variables|Spline|GetSplineCurrentTime) "World" (Variables|Spline|GetConstant%20Velocity)) 5e+01 12 "(R=1.000000,G=0.000000,B=0.000000,A=1.000000)" 0.0)
    (Rendering|Debug|DrawDebugSphere (Spline|GetLocationatTime (Variables|Default|GetSplinePlayer) (Variables|Spline|GetSplineDesiredTime) "World" (Variables|Spline|GetConstant%20Velocity)) 5e+01 12 "(R=1.000000,G=0.000000,B=0.000000,A=1.000000)" 0.0)
    (Rendering|Debug|DrawDebugSphere (Spline|GetLocationatTime (Variables|Default|GetSplineCamera) (Variables|Spline|GetSplineCurrentTime) "World" (Variables|Spline|GetConstant%20Velocity)) 5e+01 12 "(R=0.000000,G=0.045587,B=1.000000,A=1.000000)" 0.0)
    (Rendering|Debug|DrawDebugSphere (Spline|GetLocationatTime (Variables|Default|GetSplineCamera) (Variables|Spline|GetSplineDesiredTime) "World" (Variables|Spline|GetConstant%20Velocity)) 5e+01 12 "(R=0.000000,G=0.262732,B=1.000000,A=1.000000)" 0.0)))